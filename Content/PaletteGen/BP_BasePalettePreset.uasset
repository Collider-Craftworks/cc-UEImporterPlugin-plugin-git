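; Base palette preset that derives one of five palette colors, by index, from a primary and a secondary color.
; Indices 0–2 build on the primary and 3–4 on the secondary, with 1 and 4 adding no offset.
; The others add per-slot HSV offsets, clamping hue rather than wrapping it.
; A flag can instead make color 3 the HSV midpoint of the unmodified primary and secondary inputs.
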(fn `Process`
  (params (PrimaryColor :type "LinearColor Structure") (SecondaryColor :type "LinearColor Structure") (Index :type Integer))
  (returns (ReturnValue :type "LinearColor Structure"))
  (bind (_h _s _v) (`KismetMathLibrary.RGBToHSV` (select `int` Index :`0` PrimaryColor :`1` PrimaryColor :`2` PrimaryColor :`3` SecondaryColor :`4` SecondaryColor)))
  (return (`KismetMathLibrary.SelectColor` (`KismetMathLibrary.LinearColorLerpUsingHSV` (`local.PrimaryColor`) (`local.SecondaryColor`) 0.5) (`KismetMathLibrary.HSVToRGB` (`KismetMathLibrary.FClamp` (+ _h (select `int` (`local.Index`) :`0` (`self.Color0_Hue`) :`1` 0.0 :`2` (`self.Color2_Hue`) :`3` (`self.Color3_Hue`) :`4` 0.0)) 0.0 360.0) (`KismetMathLibrary.FClamp` (+ _s (select `int` (`local.Index`) :`0` (`self.Color0_Saturation`) :`1` 0.0 :`2` (`self.Color2_Saturation`) :`3` (`self.Color3_Saturation`) :`4` 0.0))) (`KismetMathLibrary.FClamp` (+ _v (select `int` (`local.Index`) :`0` (`self.Color0_Value`) :`1` 0.0 :`2` (`self.Color2_Value`) :`3` (`self.Color3_Value`) :`4` 0.0)))) (and (`self.bColor3InterpFrom2And4`) (== (`local.Index`) 3)))))